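; AK47 muzzle flash Blueprint that pairs a Niagara muzzle effect with a blinking point light.
; The construction script passes loop duration and color to the Niagara system and applies the same color to the light.
; From BeginPlay, a timeline drives light intensity, then replays after a delay equal to the Niagara loop duration, so the flash repeats continuously.
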(event EventBeginPlay
  (Components|Timeline|PlayfromStart (Variables|Default|GetfireBlinkAnimation)))

(event Collision|EventActorBeginOverlap
  (params (OtherActor :type Actor%20Object%20Reference)))

(event EventTick
  (params (DeltaSeconds :type Float%20%28single-precision%29)))

(fn ConstructionScript
  (bind _color_ak47_muzzle_set (Variables|Default|GetColor_AK47_Muzzle_set))
  (bind _niagara_muzzle (Variables|Default|GetNiagara_Muzzle))
  (Effects|Components|ParticleSystem|SetFloatParameter _niagara_muzzle "NS_AK47_LoopDuration" (Variables|Default|GetNS_AK47_LoopDuration))
  (Niagara|SetNiagaraVariable(LinearColor) _niagara_muzzle "Color_AK47_Muzzle" _color_ak47_muzzle_set)
  (Rendering|Components|Light|SetLightColor (Variables|Default|GetPointLight) _color_ak47_muzzle_set true))